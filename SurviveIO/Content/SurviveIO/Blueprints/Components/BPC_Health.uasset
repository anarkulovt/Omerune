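; BPC_Health is an actor component that tracks its owner's health in SurviveIO.
; SetDamage subtracts damage from Health, clamps it between zero and MaxHealth, then calls PrintHP to show the owner's name and current value on screen.
; PrintHP also runs on BeginPlay, and IsAlive reports whether Health is above zero.
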(event `self.ReceiveBeginPlay`
  (`self.PrintHP`))

(fn `IsAlive`
  (returns (isAlive :type Boolean))
  (return (> (`self.Health`) 0.0)))

(fn `PrintHP`
  (`KismetSystemLibrary.PrintString` (`KismetStringLibrary.BuildString_Double` (`KismetSystemLibrary.GetDisplayName` (`self.GetOwner`)) " Health = " (`self.Health`)) true true (`self.Text Color`) 5.0))

(fn `SetDamage`
  (params (Damage :type "Float (double-precision)"))
  (set `self.Health` (`KismetMathLibrary.FClamp` (- (`self.Health`) Damage) 0.0 (`self.MaxHealth`)))
  (`self.PrintHP`))