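; BP_MainHero is the player hero character, with a melee-style attack, health and a floating health bar.
; The attack input sphere-traces ahead for WorldDynamic objects, with debug drawing, and damages only the first hit.
; Incoming damage feeds BPC_Health, whose death event ragdolls the mesh and disables capsule collision; stop-movement and disable-input nodes are unwired.
; The health bar widget binds to that component on BeginPlay and faces the camera every Tick.
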(event `EnhancedInput|/Game/SurviveIO/Input/IA_Attack`
  (params (ActionValue :type Boolean) (ElapsedSeconds :type "Float (double-precision)") (TriggeredSeconds :type "Float (double-precision)") (InputAction :type "InputAction Object Reference" :default "/Game/SurviveIO/Input/IA_Attack.IA_Attack"))
  (bind _returnvalue (`self.K2_GetActorLocation`))
  (:`Triggered`
    (bind (_outhits _returnvalue_2) (`KismetSystemLibrary.SphereTraceMultiForObjects` :`Start` _returnvalue :`End` (+ _returnvalue (* (`self.GetActorForwardVector`) 200.0)) :`Radius` 200.0 :`ObjectTypes` (`|MakeArray` "ObjectTypeQuery2" :!type "EObjectTypeQuery Enum") :`DrawDebugType` "ForDuration"))
    (if _returnvalue_2
      (`GameplayStatics.ApplyDamage` (`.HitActor` (`GameplayStatics.BreakHitResult` (`|GetArrayItem` _outhits))) 20.0 (`self.GetController`) self))))

(event `self.ReceiveAnyDamage`
  (params (Damage :type "Float (single-precision)") (DamageType :type "DamageType Object Reference") (InstigatedBy :type "Controller Object Reference") (DamageCauser :type "Actor Object Reference"))
  (`/Game/SurviveIO/Blueprints/Components/BPC_Health.SetDamage` (`self.BPC_Health`) Damage))

(event `self.BPC_Health.OnDeath`
  (set `self.bCanBeDamaged` false)
  (`PrimitiveComponent.SetCollisionProfileName` (`self.Mesh`) "PhysicsActor" true)
  (`PrimitiveComponent.SetCollisionEnabled` (`self.CapsuleComponent`) "NoCollision")
  (`PrimitiveComponent.SetSimulatePhysics` (`self.Mesh`) true)
  (`KismetSystemLibrary.PrintString` "DEAD" true true (struct :`R` 1.0 :`G` 0.024173 :`B` 0.101132 :`A` 1.0) 5.0))

(event `self.ReceiveTick`
  (params (DeltaSeconds :type "Float (single-precision)"))
  (`SceneComponent.K2_SetWorldRotation` (`self.HealthbarWidget`) (`KismetMathLibrary.FindLookAtRotation` (`SceneComponent.K2_GetComponentLocation` (`self.HealthbarWidget`)) (`SceneComponent.K2_GetComponentLocation` (`PlayerCameraManager.TransformComponent` (`GameplayStatics.GetPlayerCameraManager` 0)))) false false))

(event `self.ReceiveBeginPlay`
  (bind _aswbp_health_bar (cast `/Game/SurviveIO/UI/WBP_HealthBar` (`WidgetComponent.GetUserWidgetObject` (`self.HealthbarWidget`))))
  (`/Game/SurviveIO/UI/WBP_HealthBar.InitHealthBar` _aswbp_health_bar (`self.BPC_Health`)))

(fn `UserConstructionScript`
  (`parent.UserConstructionScript`))