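; Game mode for SurviveIO, a timed survival match that is won when the countdown runs out and lost when the player dies.
; On begin play it starts a one-second countdown and activates every BP_Spawner, binding spawned enemies' health death events to add score to GS_SurviveIO.
; The spawned player pawn's death event is also bound.
; Both outcomes show WBP_GameOver with win and high-score flags, but only game over stops the spawners.
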(event `self.ReceiveBeginPlay`
  (bind _returnvalue (`KismetSystemLibrary.K2_SetTimerDelegate` (delegate `CountDown`) 1.0 true))
  (`self.GetSpawners`))

(event `CountDown`
  (bind _output_get (set `self.TimeRemaining` (- (`self.TimeRemaining`) 1.0)))
  (if (<= _output_get 0.0)
    (`KismetSystemLibrary.K2_ClearAndInvalidateTimerHandle` (stale `self.ReceiveBeginPlay` _returnvalue))
    (`self.ShowGameState` true)))

(event `GetSpawners`
  (bind _outactors (`GameplayStatics.GetAllActorsOfClass` "/Game/SurviveIO/Blueprints/BP_Spawner.BP_Spawner_C"))
  (for _array_element _outactors
    (`/Game/SurviveIO/Blueprints/BP_Spawner.OnGameStart` _array_element)
    (add `/Game/SurviveIO/Blueprints/BP_Spawner.OnEnemySpawn` _array_element (delegate `OnEnemySpawn`))))

(event `OnEnemySpawn`
  (params (SpawnedActor :type "Actor Object Reference"))
  (add `/Game/SurviveIO/Blueprints/Components/BPC_Health.OnDeath` (`self.GetComponentByClass` SpawnedActor "/Game/SurviveIO/Blueprints/Components/BPC_Health.BPC_Health_C") (delegate `OnEnemyDeath`)))

(event `OnEnemyDeath`
  (bind _asgs_survive_io (cast `/Game/SurviveIO/Blueprints/GS_SurviveIO` (`GameplayStatics.GetGameState`)))
  (`/Game/SurviveIO/Blueprints/GS_SurviveIO.AddScore` _asgs_survive_io 20.0))

(event `OnPlayerDeath`
  (`self.OnGameOver`))

(event `OnGameOver`
  (`self.ShowGameState` false)
  (bind _outactors (`GameplayStatics.GetAllActorsOfClass` "/Game/SurviveIO/Blueprints/BP_Spawner.BP_Spawner_C"))
  (for _array_element _outactors
    (`/Game/SurviveIO/Blueprints/BP_Spawner.OnGameEnd` _array_element)))

(event `ShowGameState`
  (params (isWin :type Boolean))
  (bind _asgs_survive_io (cast `/Game/SurviveIO/Blueprints/GS_SurviveIO` (`GameplayStatics.GetGameState`)))
  (bind _returnvalue (`|CreateWidget` "/Game/SurviveIO/UI/WBP_GameOver.WBP_GameOver_C" (`GameplayStatics.GetPlayerController` 0) isWin (`/Game/SurviveIO/Blueprints/GS_SurviveIO.isHighscore` _asgs_survive_io)))
  (`UserWidget.AddToViewport` _returnvalue 0))

(fn `SpawnDefaultPawnAtTransform`
  (params (NewPlayer :type "Controller Object Reference") (SpawnTransform :type "Transform Structure (by ref)"))
  (returns (ReturnValue :type "Pawn Object Reference"))
  (bind _returnvalue (`parent.SpawnDefaultPawnAtTransform` NewPlayer SpawnTransform))
  (add `/Game/SurviveIO/Blueprints/Components/BPC_Health.OnDeath` (`self.GetComponentByClass` _returnvalue "/Game/SurviveIO/Blueprints/Components/BPC_Health.BPC_Health_C") (`|CreateDelegate` :!event `OnPlayerDeath`))
  (return _returnvalue))

(fn `UserConstructionScript`)