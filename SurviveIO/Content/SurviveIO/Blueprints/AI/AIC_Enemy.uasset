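; AI controller for enemies that finds a nearby pawn, chases it and attacks.
; Each tick, while the controlled pawn is alive and has no target, a forward multi-sphere trace takes the first pawn hit and starts AIMoveTo toward it.
; Arrival triggers BP_Enemy's Attack and clears CanMove for a delay, then restores it and releases the target to resume searching; a failed move releases it immediately.
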(event `self.ReceiveTick`
  (params (DeltaSeconds :type "Float (single-precision)"))
  (bind _returnvalue (`self.K2_GetPawn`))
  (bind _returnvalue_2 (`self.K2_GetPawn`))
  (bind _returnvalue_3 (`self.K2_GetActorLocation` _returnvalue))
  (`/Engine/EditorBlueprintResources/StandardMacros.IsValid` _returnvalue_2
    (:`Is Valid`
      (if (`/Game/SurviveIO/Blueprints/Components/BPC_Health.IsAlive` (`self.GetComponentByClass` _returnvalue_2 "/Game/SurviveIO/Blueprints/Components/BPC_Health.BPC_Health_C"))
        (`self.hasTarget`
          (:`then`)
          (:`else`
            (bind (_outhits _returnvalue_4) (`KismetSystemLibrary.SphereTraceMultiForObjects` :`Start` _returnvalue_3 :`End` (+ _returnvalue_3 (* (`self.GetActorForwardVector` _returnvalue) 500.0)) :`Radius` 400.0 :`ObjectTypes` (`|MakeArray` "ObjectTypeQuery3" :!type "EObjectTypeQuery Enum") :`DrawDebugType` "ForOneFrame"))
            (if _returnvalue_4
              (set `self.hasTarget` true)
              (bind _output_get (set `self.Target` (`.HitActor` (`GameplayStatics.BreakHitResult` (`|GetArrayItem` _outhits)))))
              (`|AIMoveTo` (`self.K2_GetPawn`) (0.0 0.0 0.0) _output_get 80.0 true
                (:`OnSuccess`
                  (`self.AttackTarget`))
                (:`OnFail`
                  (set `self.hasTarget` false))))))))))

(event `AttackTarget`
  (bind _asbp_enemy (cast `/Game/SurviveIO/Blueprints/Characters/BP_Enemy` (`self.K2_GetPawn`)))
  (`/Game/SurviveIO/Blueprints/Characters/BP_Enemy.Attack` _asbp_enemy)
  (set `/Game/SurviveIO/Blueprints/Characters/BP_Enemy.canMove` false _asbp_enemy)
  (`KismetSystemLibrary.Delay` (`self.AttackDelay`))
  (set `self.hasTarget` false)
  (set `/Game/SurviveIO/Blueprints/Characters/BP_Enemy.canMove` true _asbp_enemy))

(fn `UserConstructionScript`)