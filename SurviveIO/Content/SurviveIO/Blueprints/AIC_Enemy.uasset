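; AI controller for enemies that finds a pawn in front of it, chases it and deals damage.
; While its pawn is alive per BPC_Health, Tick runs a forward sphere trace for Pawn objects whenever it has no target.
; The first hit becomes the AI MoveTo goal; arrival applies damage, then a delay clears the target flag.
; A failed move clears the flag immediately.
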(event `self.ReceiveTick`
  (params (DeltaSeconds :type "Float (single-precision)"))
  (bind _returnvalue (`self.K2_GetPawn`))
  (bind _returnvalue_2 (`self.K2_GetPawn`))
  (bind _returnvalue_3 (`self.K2_GetActorLocation` _returnvalue))
  (`/Engine/EditorBlueprintResources/StandardMacros.IsValid` _returnvalue_2
    (:`Is Valid`
      (if (`/Game/SurviveIO/Blueprints/Components/BPC_Health.IsAlive` (`self.GetComponentByClass` _returnvalue_2 "/Game/SurviveIO/Blueprints/Components/BPC_Health.BPC_Health_C"))
        (`self.hasTarget`
          (:`then`)
          (:`else`
            (bind (_outhits _returnvalue_4) (`KismetSystemLibrary.SphereTraceMultiForObjects` :`Start` _returnvalue_3 :`End` (+ _returnvalue_3 (* (`self.GetActorForwardVector` _returnvalue) 500.0)) :`Radius` 40.0 :`ObjectTypes` (`|MakeArray` "ObjectTypeQuery3" :!type "EObjectTypeQuery Enum") :`DrawDebugType` "ForOneFrame"))
            (if _returnvalue_4
              (set `self.hasTarget` true)
              (set `self.Target` (`.HitActor` (`GameplayStatics.BreakHitResult` (`|GetArrayItem` _outhits))))
              (`|AIMoveTo` (`self.K2_GetPawn`) (0.0 0.0 0.0) (`self.Target`) 150.0 true
                (:`OnSuccess`
                  (`self.AttackTarget`))
                (:`OnFail`
                  (set `self.hasTarget` false))))))))))

(event `AttackTarget`
  (`GameplayStatics.ApplyDamage` (`self.Target`) 20.0 self (`self.K2_GetPawn`))
  (`KismetSystemLibrary.Delay` (`self.AttackDelay`))
  (set `self.hasTarget` false))

(fn `UserConstructionScript`)