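; BP_Zombie is an AI or controller-possessed zombie in SurviveIO that takes damage and explodes on death.
; Incoming damage feeds its health component, whose death event unpossesses the controller, spawns an explosion effect and destroys the actor.
; A widget component shows a health bar bound to that component at BeginPlay and turns toward the player camera every tick.
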(event `self.ReceiveAnyDamage`
  (params (Damage :type "Float (single-precision)") (DamageType :type "DamageType Object Reference") (InstigatedBy :type "Controller Object Reference") (DamageCauser :type "Actor Object Reference"))
  (`/Game/SurviveIO/Blueprints/Components/BPC_Health.SetDamage` (`self.BPC_Health`) Damage))

(event `self.BPC_Health.OnDeath`
  (`Controller.UnPossess` (`self.GetController`))
  (`GameplayStatics.SpawnEmitterAtLocation` "/Game/StarterContent/Particles/P_Explosion.P_Explosion" (`self.K2_GetActorLocation`))
  (`self.K2_DestroyActor`))

(event `self.ReceiveTick`
  (params (DeltaSeconds :type "Float (single-precision)"))
  (`SceneComponent.K2_SetWorldRotation` (`self.HealthbarWidget`) (`KismetMathLibrary.FindLookAtRotation` (`SceneComponent.K2_GetComponentLocation` (`self.HealthbarWidget`)) (`SceneComponent.K2_GetComponentLocation` (`PlayerCameraManager.TransformComponent` (`GameplayStatics.GetPlayerCameraManager` 0)))) false false))

(event `self.ReceiveBeginPlay`
  (bind _aswbp_health_bar (cast `/Game/SurviveIO/UI/WBP_HealthBar` (`WidgetComponent.GetUserWidgetObject` (`self.HealthbarWidget`))))
  (`/Game/SurviveIO/UI/WBP_HealthBar.InitHealthBar` _aswbp_health_bar (`self.BPC_Health`)))

(fn `UserConstructionScript`)