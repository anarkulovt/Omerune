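; GS_SurviveIO is the game state for SurviveIO, tracking the current score and a persistent high score.
; On BeginPlay it loads the SG_SurviveIO save and reads its high score, or creates a save object if none exists.
; AddScore fires the ScoreChanged dispatcher, and whenever the high score is beaten it sets IsHighscore and immediately writes the save slot.
; Loading and saving report through debug prints.
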(event `self.ReceiveBeginPlay`
  (bind _returnvalue (`GameplayStatics.DoesSaveGameExist` (`self.Slot Name`)))
  (if _returnvalue
    (bind _returnvalue_2 (`GameplayStatics.LoadGameFromSlot` (`self.Slot Name`)))
    (bind _output_get (set `self.SaveGame` _returnvalue_2))
    (bind _assg_survive_io (cast `/Game/SurviveIO/Blueprints/Framework/SG_SurviveIO` _output_get))
    (bind _output_get_2 (set `self.HighScore` (`/Game/SurviveIO/Blueprints/Framework/SG_SurviveIO.HighScore` _assg_survive_io)))
    (`KismetSystemLibrary.PrintString` (`KismetStringLibrary.BuildString_Double` "" "Current Highscore = " _output_get_2) true true (struct :`G` 1.0 :`B` 0.723777 :`A` 1.0) 5.0)
    (else
      (bind _returnvalue_3 (`GameplayStatics.CreateSaveGameObject` "/Game/SurviveIO/Blueprints/Framework/SG_SurviveIO.SG_SurviveIO_C"))
      (set `self.SaveGame` _returnvalue_3))))

(event `AddScore`
  (params (Score :type "Float (double-precision)"))
  (set `self.CurrentScore` (+ (`self.CurrentScore`) Score))
  (`self.ScoreChanged`)
  (if (> (`self.CurrentScore`) (`self.HighScore`))
    (set `self.HighScore` (`self.CurrentScore`))
    (set `self.isHighscore` true)
    (`self.SaveHighscore`)))

(event `SaveHighscore`
  (bind _assg_survive_io (cast `/Game/SurviveIO/Blueprints/Framework/SG_SurviveIO` (`self.SaveGame`)))
  (set `/Game/SurviveIO/Blueprints/Framework/SG_SurviveIO.HighScore` (`self.HighScore`) _assg_survive_io)
  (bind _returnvalue (`GameplayStatics.SaveGameToSlot` _assg_survive_io (`self.Slot Name`)))
  (if _returnvalue
    (`KismetSystemLibrary.PrintString` "Highscore saved" true true (struct :`R` 0.668275 :`G` 1.0 :`B` 0.400563 :`A` 1.0) 10.0)
    (else
      (`KismetSystemLibrary.PrintString` "Can't save highscore" true true (struct :`R` 1.0 :`G` 0.152994 :`B` 0.237288 :`A` 1.0) 10.0))))

(fn `UserConstructionScript`)