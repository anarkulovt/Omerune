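; GM_SurviveIO is the game mode for SurviveIO, running the spawner lifecycle, score and game over.
; On BeginPlay it starts every BP_Spawner and hooks each spawned enemy's BPC_Health death event to add to the score.
; An overridden SpawnDefaultPawnAtTransform binds the player pawn's death event at spawn.
; Player death triggers game over, which stops all spawners; score and game over only print to screen.
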(event `self.ReceiveBeginPlay`
  (bind _outactors (`GameplayStatics.GetAllActorsOfClass` "/Game/SurviveIO/Blueprints/BP_Spawner.BP_Spawner_C"))
  (for _array_element _outactors
    (`/Game/SurviveIO/Blueprints/BP_Spawner.OnGameStart` _array_element)
    (add `/Game/SurviveIO/Blueprints/BP_Spawner.OnEnemySpawn` _array_element (delegate `OnEnemySpawn`))))

(event `OnEnemySpawn`
  (params (SpawnedActor :type "Actor Object Reference"))
  (add `/Game/SurviveIO/Blueprints/Components/BPC_Health.OnDeath` (`self.GetComponentByClass` SpawnedActor "/Game/SurviveIO/Blueprints/Components/BPC_Health.BPC_Health_C") (delegate `OnEnemyDeath`)))

(event `OnEnemyDeath`
  (bind _output_get (set `self.CurrentScore` (+ (`self.CurrentScore`) 20.0)))
  (`KismetSystemLibrary.PrintString` (`KismetStringLibrary.BuildString_Double` "" "Current Score = " _output_get) true true (struct :`G` 0.66 :`B` 1.0 :`A` 1.0) 5.0))

(event `self.K2_PostLogin`
  (params (NewPlayer :type "PlayerController Object Reference")))

(event `OnPlayerDeath`
  (`self.OnGameOver`))

(event `OnGameOver`
  (`KismetSystemLibrary.PrintString` "GAME OVER" true true (struct :`R` 1.0 :`G` 0.461935 :`B` 0.058952 :`A` 1.0) 10.0)
  (bind _outactors (`GameplayStatics.GetAllActorsOfClass` "/Game/SurviveIO/Blueprints/BP_Spawner.BP_Spawner_C"))
  (for _array_element _outactors
    (`/Game/SurviveIO/Blueprints/BP_Spawner.OnGameEnd` _array_element)))

(fn `SpawnDefaultPawnAtTransform`
  (params (NewPlayer :type "Controller Object Reference") (SpawnTransform :type "Transform Structure (by ref)"))
  (returns (ReturnValue :type "Pawn Object Reference"))
  (bind _returnvalue (`parent.SpawnDefaultPawnAtTransform` NewPlayer SpawnTransform))
  (add `/Game/SurviveIO/Blueprints/Components/BPC_Health.OnDeath` (`self.GetComponentByClass` _returnvalue "/Game/SurviveIO/Blueprints/Components/BPC_Health.BPC_Health_C") (`|CreateDelegate` :!event `OnPlayerDeath`))
  (return _returnvalue))

(fn `UserConstructionScript`)